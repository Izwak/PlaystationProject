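; Base projectile class that damages and knocks back players and enemies on hit, then destroys itself, or after a two-second check in Tick.
; Actor X scale sets damage and player knockback force, and projectiles at 0.3 or below destroy on any hit.
; SwitchDir parries by flipping yaw based on the player's Y side and relaunching forward and up.
; WallHit and OnParryEvent are empty hooks, and the Shooter check has no effect.
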(event OnComponentHit(Collider)
  (params (HitComponent :type Primitive%20Component%20Object%20Reference) (OtherActor :type Actor%20Object%20Reference) (OtherComp :type Primitive%20Component%20Object%20Reference) (NormalImpulse :type Vector :default "0, 0, 0") (Hit :type Hit%20Result%20Structure%20%28by%20ref%29))
  (bind _return_value_x (CallFunction|GetSize))
  (bind _location (Collision|BreakHitResult Hit))
  (bind _returnvalue (* 2e+01 _return_value_x))
  ;[1 1 1] Projectile
  (if (> (CallFunction|GetSize) 0.3)
    (if (!= (Variables|Default|GetShooter) OtherActor)
      _
      (else
        _))
    (bind _asmy_character (Utilities|Casting|CastTomyCharacter OtherActor)
      (:then
        (CallFunction|DamagePlayer _asmy_character _returnvalue _location)
        (Actor|DestroyActor :!label _label))
      (:CastFailed
        (bind _asbase_enemy_class (Utilities|Casting|CastToBaseEnemyClass OtherActor)
          (:then
            (CallFunction|DamageEnemy _asbase_enemy_class _returnvalue _location)
            (goto _label))
          (:CastFailed
            (CallFunction|WallHit)))))
    (else
      (goto _label))))

(event Custom|SetVelocity
  (params (Velocity :type Vector))
  ;[1 1 1] Set Velocity
  (Variables|/Script/Engine.MovementComponent|SetVelocity (Variables|Default|GetProjectileMovement) Velocity)
  (Development|PrintString "Set Vel"))

(event Custom|Wall%20Hit)

(event Custom|OnParryEvent)

(event Custom|DamagePlayer
  (params (Player :type My%20Character%20Object%20Reference) (Damage :type Float%20%28double-precision%29) (Hit%20Pos :type Vector))
  ;[1 1 1] Damage Player
  (Game|Damage|ApplyDamage Player Damage 0 0)
  (Default|Knockback Player Hit%20Pos (* 9e+02 (CallFunction|GetSize))))

(event Custom|Damage%20Enemy
  (params (Enemy :type Base%20Enemy%20Class%20Object%20Reference) (Damage :type Float%20%28single-precision%29) (InputPin :type Vector))
  ;[1 1 1] Damage Enemy
  (Game|Damage|ApplyDamage Enemy Damage 0 0)
  (Default|Knockback Enemy (Transformation|GetVelocity) InputPin))

(event Custom|TerminateBall
  ;[1 1 1] Terminate Ball
  (if (> (Class|KismetMathLibrary|GetSecond) 2)
    (Actor|DestroyActor)))

(event Custom|SwitchDir
  (params (PlayerPos :type Vector))
  (bind _returnvalue (Transformation|GetActorRotation))
  (bind _returnvalue_2 (Transformation|GetActorRotation))
  (bind _returnvalue_3 (> (.yaw _returnvalue) 0.0))
  ;[1 1 1] Force A bounce in the oppisite Direction
  (if (> (.y PlayerPos) (.y (Transformation|GetActorLocation)))
    (if _returnvalue_3
      (Transformation|SetActorRotation (Math|Rotator|MakeRotator (.roll _returnvalue_2) (.pitch _returnvalue_2) (* (.yaw _returnvalue_2) -1.0)) :!label _label)
      (CallFunction|OnParryEvent)
      (Variables|/Script/Engine.MovementComponent|SetVelocity (Variables|Default|GetProjectileMovement) (+ (* (Transformation|GetActorForwardVector) 8e+02) (* (Transformation|GetActorUpVector) 1.1e+03))))
    (elif (not _returnvalue_3)
      (goto _label))))

(event EventTick
  (params (DeltaSeconds :type Float%20%28single-precision%29))
  ;[1 1 1] Setup
  (CallFunction|TerminateBall))

(fn ConstructionScript)

(fn GetSize
  (return (.x (Transformation|GetActorScale3D))))