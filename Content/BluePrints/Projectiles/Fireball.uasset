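; Fireball projectile Blueprint that shrinks over its lifetime, extending a parent class that supplies a parry event.
; A timeline starts on BeginPlay and scales the actor uniformly through its Size track.
; The parry event restarts that timeline from the beginning, resetting the scale curve.
; A separate Terminate event destroys the actor when size is zero or below, with no caller shown in the graph.
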(event Custom|Terminate
  ;[1 1 1] Terminate Ball
  (if (not (> (CallFunction|GetSize) 0.0))
    (Actor|DestroyActor)))

(event Custom|ScaleDown
  ;[1 1 1] Scale Down
  (bind _size (Timeline|Timeline_1 PlayFromStart)
    (:Update
      (Transformation|SetActorScale3D (* (Class|KismetMathLibrary|VectorOne) _size)))))

(event EventBeginPlay
  (|CallParentFunction)
  (CallFunction|ScaleDown))

(event Collision|EventActorBeginOverlap
  (params (OtherActor :type Actor%20Object%20Reference)))

(event EventTick
  (params (DeltaSeconds :type Float%20%28single-precision%29))
  (|CallParentFunction DeltaSeconds) ; This node is disabled and will not be called.\nDrag off pins to build functionality.
)

(event EventOnParryEvent
  ;[1 1 1] Scale Down
  (bind _size (Timeline|Timeline_1 PlayFromStart)
    (:Update
      (Transformation|SetActorScale3D (* (Class|KismetMathLibrary|VectorOne) _size)))))

(fn ConstructionScript
  (|CallParentFunction))