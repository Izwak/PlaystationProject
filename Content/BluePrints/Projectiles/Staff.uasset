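; Thrown staff projectile that bounces around on a plane locked to its starting X, damaging and knocking back enemies it hits.
; Tick spins the mesh, alternating direction with each bounce, until the fifth bounce alters projectile movement to settle it and enables gravity.
; It destroys itself and calls ShowStaff on the player when it falls into the void, hits the player, or is near them after a short delay.
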(event OnComponentHit(Sphere)
  (params (HitComponent :type Primitive%20Component%20Object%20Reference) (OtherActor :type Actor%20Object%20Reference) (OtherComp :type Primitive%20Component%20Object%20Reference) (NormalImpulse :type Vector :default "0, 0, 0") (Hit :type Hit%20Result%20Structure%20%28by%20ref%29))
  (bind _bounces (Variables|Default|Getbounces))
  ;[1 1 1] Staff Hit
  (if (> (Variables|Default|Gettimer) 0.05)
    (Math|Integer|IncrementInt _bounces
      (:%20%20
        (if (== _bounces 5)
          (CallFunction|StopStaff)
          (else
            (Development|PrintString "Stick Collision")
            (bind _asbase_enemy_class (Utilities|Casting|CastToBaseEnemyClass OtherActor)
              (:then
                (Game|Damage|ApplyDamage _asbase_enemy_class 1e+01 0 0)
                (Default|Knockback _asbase_enemy_class "0, 0, 0" (.ImpactPoint (Collision|BreakHitResult Hit))))
              (:CastFailed
                (bind _asmy_character (Utilities|Casting|CastTomyCharacter OtherActor))
                (Default|ShowStaff _asmy_character)
                (Actor|DestroyActor)))))))))

(event Custom|Set%20Movement
  (params (StartingVel :type Vector))
  ;[1 1 1] Setup
  (bind _output_get (Variables|/Script/Engine.MovementComponent|SetVelocity (Variables|Default|GetProjectileMovement) StartingVel))
  (Development|PrintString (Utilities|String|ToString(Vector) _output_get) true true "(R=0.378884,G=0.000000,B=1.000000,A=1.000000)"))

(event Custom|Stop%20Staff
  (bind _returnvalue (Transformation|GetVelocity))
  (bind _projectilemovement (Variables|Default|GetProjectileMovement))
  ;[1 1 1] Stop Staff
  (Variables|/Script/Engine.MovementComponent|SetVelocity _projectilemovement (Math|Vector|MakeVector (.x _returnvalue) 1.0 (.z _returnvalue)))
  (Variables|/Script/Engine.ProjectileMovementComponent|SetBounciness _projectilemovement 0.5)
  (Variables|/Script/Engine.ProjectileMovementComponent|SetFriction _projectilemovement 1.0)
  (Physics|SetEnableGravity (Variables|Default|GetSphere) true))

(event Custom|Overlap%20Collision
  (bind _returnvalue (Transformation|GetVelocity))
  ;[1 1 1] Overlap Collision
  (if (and (== (* (.x _returnvalue) (.y _returnvalue) (.z _returnvalue)) 0.0) (>= (Variables|Default|Getbounces) 5))
    _))

(event Custom|Set%20Staff%20Spin
  (bind _bounces (Variables|Default|Getbounces))
  (bind _cube (Variables|Default|GetCube))
  (bind _returnvalue (Transformation|GetWorldRotation _cube))
  ;[1 1 1] Set Staff Spin
  (if (< _bounces 5)
    (if (== (Math|Integer|%(Integer) _bounces 2) 0)
      (Variables|Default|SetSpinDir 1)
      (else
        (Variables|Default|SetSpinDir -1)))
    (Transformation|SetWorldRotation (Variables|Default|GetCube) (Math|Rotator|MakeRotator (+ (.roll _returnvalue) (* (Variables|Default|GetdeltaSeconds) 5e+02 (Variables|Default|GetSpinDir))) 0.0 0.0) false false)
    (else
      (Transformation|SetWorldRotation (Variables|Default|GetCube) (Math|Rotator|Lerp(Rotator) (Math|Rotator|MakeRotator (.roll _returnvalue) (.pitch _returnvalue) (.yaw _returnvalue)) "0, 0, 0" 0.5) false false))))

(event Custom|Check%20Distance
  (bind _returnvalue (Transformation|GetActorLocation))
  ;[1 1 1] Check Fallem into Void
  (bind _asmy_character (Utilities|Casting|CastTomyCharacter (Game|GetPlayerCharacter 0)))
  (if (< (.z _returnvalue) -1e+04)
    (Default|ShowStaff _asmy_character :!label _label)
    (Actor|DestroyActor)
    (elif (and (< (Math|Vector|Distance(Vector) (Math|Vector|MakeVector (.x _returnvalue) (.y _returnvalue) (.z _returnvalue)) (Transformation|GetActorLocation _asmy_character)) 3e+02) (> (Variables|Default|Gettimer) 1.0))
      (goto _label))))

(event EventBeginPlay
  ;[1 1 1] Tick / Begin
  (Variables|Default|SetstartingX (.x (Transformation|GetActorLocation))))

(event EventTick
  (params (DeltaSeconds :type Float%20%28single-precision%29))
  (bind _returnvalue (Transformation|GetActorLocation))
  ;[1 1 1] Tick / Begin
  (bind _output_get (Variables|Default|SetdeltaSeconds DeltaSeconds))
  (Variables|Default|Settimer (+ _output_get (Variables|Default|Gettimer)))
  (Transformation|SetActorLocation (Math|Vector|MakeVector (Variables|Default|GetstartingX) (.y _returnvalue) (.z _returnvalue)) false false)
  (CallFunction|OverlapCollision)
  (CallFunction|SetStaffSpin)
  (CallFunction|CheckDistance))

(fn ConstructionScript)