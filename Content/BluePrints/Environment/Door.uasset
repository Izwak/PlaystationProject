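; Interactive hinged door that swings away from the player and closes when they leave its trigger box.
; Box overlap by myCharacter toggles input, and the Special action drives a FlipFlop between opening and closing.
; A world Y comparison between player and Door2 picks one of two yaw timelines, reversed to close.
; HingeDir stores the swing direction, and a non-zero value on end overlap re-enters the FlipFlop to close the door.
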(event OnComponentBeginOverlap(Box)
  (params (OverlappedComponent :type Primitive%20Component%20Object%20Reference) (OtherActor :type Actor%20Object%20Reference) (OtherComp :type Primitive%20Component%20Object%20Reference) (OtherBodyIndex :type Integer) (bFromSweep :type Boolean) (SweepResult :type Hit%20Result%20Structure%20%28by%20ref%29))
  ;[1 1 1] Door
  ;;[1 1 1] Open Button Enabled When Close to Door
  (Utilities|Casting|CastTomyCharacter OtherActor)
  (Input|EnableInput (Game|GetPlayerController 0)))

(event OnComponentEndOverlap(Box)
  (params (OverlappedComponent :type Primitive%20Component%20Object%20Reference) (OtherActor :type Actor%20Object%20Reference) (OtherComp :type Primitive%20Component%20Object%20Reference) (OtherBodyIndex :type Integer))
  (bind _returnvalue (Game|GetPlayerCharacter 0))
  (bind _door2 (Variables|Default|GetDoor2))
  (bind _door2_2 (Variables|Default|GetDoor2))
  (bind _returnvalue_2 (Transformation|GetWorldLocation _door2))
  (bind _rootcomponent (Variables|/Script/Engine.Actor|GetRootComponent _returnvalue))
  (bind _returnvalue_3 (Transformation|GetWorldLocation _rootcomponent))
  (bind _returnvalue_4 (> (.y _returnvalue_3) (.y _returnvalue_2)))
  ;[1 1 1] Door
  ;;[1 1 1] Disable Open Button If Far From Door and Close if open
  (Utilities|Casting|CastTomyCharacter OtherActor)
  (Input|DisableInput (Game|GetPlayerController 0))
  (if (not (== (Variables|Default|GetHinge%20Dir) 0))
    (Utilities|FlowControl|FlipFlop
      (:A
        ;;[1 1 1] Door set to Open
        (if (== (Variables|Default|GetHinge%20Dir) 0)
          (if _returnvalue_4
            ;;[1 1 1] Pick Direction of Door Swing Away From Player
            (Variables|Default|SetHinge%20Dir 1 :!label _label)
            (bind _newtrack_0 (Timeline|Timeline_0 Play)
              (:Update
                (Transformation|SetRelativeRotation _door2_2 (Math|Rotator|MakeRotator 0.0 0.0 _newtrack_0) false false)))
            (else
              (Variables|Default|SetHinge%20Dir -1 :!label _label_2)
              (bind _newtrack_0_2 (Timeline|Timeline_1 Play)
                (:Update
                  (Transformation|SetRelativeRotation _door2_2 (Math|Rotator|MakeRotator 0.0 0.0 _newtrack_0_2) false false)))))
          (elif (> (Variables|Default|GetHinge%20Dir) 0)
            (goto _label)
            (else
              (goto _label_2)))))
      (:B
        ;;[1 1 1] Door Set to Close
        (if (== (Variables|Default|GetHinge%20Dir) 0)
          (if _returnvalue_4
            ;;[1 1 1] Allow door to Open Either Way if Door Closed
            (Variables|Default|SetHinge%20Dir 0 :!label _label_3)
            (Timeline|Timeline_0 Reverse)
            (else
              (Variables|Default|SetHinge%20Dir 0 :!label _label_4)
              (Timeline|Timeline_1 Reverse)))
          (elif (> (Variables|Default|GetHinge%20Dir) 0)
            (goto _label_3)
            (else
              (goto _label_4))))))))

(event Input|ActionEvents|InputActionSpecial
  (params (Key :type Key%20Structure))
  (bind _returnvalue (Game|GetPlayerCharacter 0))
  (bind _door2 (Variables|Default|GetDoor2))
  (bind _door2_2 (Variables|Default|GetDoor2))
  (bind _returnvalue_2 (Transformation|GetWorldLocation _door2))
  (bind _rootcomponent (Variables|/Script/Engine.Actor|GetRootComponent _returnvalue))
  (bind _returnvalue_3 (Transformation|GetWorldLocation _rootcomponent))
  (bind _returnvalue_4 (> (.y _returnvalue_3) (.y _returnvalue_2)))
  ;[1 1 1] Door
  ;;[1 1 1] Open Door Input
  (:Pressed
    (Utilities|FlowControl|FlipFlop
      (:A
        ;;[1 1 1] Door set to Open
        (if (== (Variables|Default|GetHinge%20Dir) 0)
          (if _returnvalue_4
            ;;[1 1 1] Pick Direction of Door Swing Away From Player
            (Variables|Default|SetHinge%20Dir 1 :!label _label)
            (bind _newtrack_0 (Timeline|Timeline_0 Play)
              (:Update
                (Transformation|SetRelativeRotation _door2_2 (Math|Rotator|MakeRotator 0.0 0.0 _newtrack_0) false false)))
            (else
              (Variables|Default|SetHinge%20Dir -1 :!label _label_2)
              (bind _newtrack_0_2 (Timeline|Timeline_1 Play)
                (:Update
                  (Transformation|SetRelativeRotation _door2_2 (Math|Rotator|MakeRotator 0.0 0.0 _newtrack_0_2) false false)))))
          (elif (> (Variables|Default|GetHinge%20Dir) 0)
            (goto _label)
            (else
              (goto _label_2)))))
      (:B
        ;;[1 1 1] Door Set to Close
        (if (== (Variables|Default|GetHinge%20Dir) 0)
          (if _returnvalue_4
            ;;[1 1 1] Allow door to Open Either Way if Door Closed
            (Variables|Default|SetHinge%20Dir 0 :!label _label_3)
            (Timeline|Timeline_0 Reverse)
            (else
              (Variables|Default|SetHinge%20Dir 0 :!label _label_4)
              (Timeline|Timeline_1 Reverse)))
          (elif (> (Variables|Default|GetHinge%20Dir) 0)
            (goto _label_3)
            (else
              (goto _label_4))))))))

(fn ConstructionScript)