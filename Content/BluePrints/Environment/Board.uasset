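; Board is a one-way platform that the player can jump up through from below or drop through from on top.
; DownBox sets the character's FallThroughFloor to Ignore while overlapped and back to Block on exit.
; UpBox enables the board's input, so Jump with down held cancels the jump, ignores the floor and starts Falling.
; Leaving UpBox restores blocking and disables input only when the IsUnder flag from DownBox is clear.
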(event OnComponentBeginOverlap(DownBox)
  (params (OverlappedComponent :type Primitive%20Component%20Object%20Reference) (OtherActor :type Actor%20Object%20Reference) (OtherComp :type Primitive%20Component%20Object%20Reference) (OtherBodyIndex :type Integer) (bFromSweep :type Boolean) (SweepResult :type Hit%20Result%20Structure%20%28by%20ref%29))
  ;[1 1 1] Go up through floor
  (bind _asmy_character (Utilities|Casting|CastTomyCharacter OtherActor))
  (bind _output_get (Variables|Default|SetPlayer _asmy_character))
  (Default|FallThroughFloor _output_get "ECR_Ignore")
  (Variables|Default|SetisUnder true))

(event OnComponentEndOverlap(DownBox)
  (params (OverlappedComponent :type Primitive%20Component%20Object%20Reference) (OtherActor :type Actor%20Object%20Reference) (OtherComp :type Primitive%20Component%20Object%20Reference) (OtherBodyIndex :type Integer))
  ;[1 1 1] Go up through floor
  (bind _asmy_character (Utilities|Casting|CastTomyCharacter OtherActor))
  (Default|FallThroughFloor _asmy_character "ECR_Block")
  (Variables|Default|SetisUnder false))

(event OnComponentBeginOverlap(UpBox)
  (params (OverlappedComponent :type Primitive%20Component%20Object%20Reference) (OtherActor :type Actor%20Object%20Reference) (OtherComp :type Primitive%20Component%20Object%20Reference) (OtherBodyIndex :type Integer) (bFromSweep :type Boolean) (SweepResult :type Hit%20Result%20Structure%20%28by%20ref%29))
  ;[1 1 1] Set whether you can fall through floor
  (bind _asmy_character (Utilities|Casting|CastTomyCharacter OtherActor))
  (Variables|Default|SetPlayer _asmy_character)
  (Input|EnableInput (Game|GetPlayerController 0)))

(event OnComponentEndOverlap(UpBox)
  (params (OverlappedComponent :type Primitive%20Component%20Object%20Reference) (OtherActor :type Actor%20Object%20Reference) (OtherComp :type Primitive%20Component%20Object%20Reference) (OtherBodyIndex :type Integer))
  ;[1 1 1] Set whether you can fall through floor
  (if (not (Variables|Default|GetisUnder))
    (bind _asmy_character (Utilities|Casting|CastTomyCharacter OtherActor))
    (Default|FallThroughFloor _asmy_character "ECR_Block")
    (Input|DisableInput (Game|GetPlayerController 0))))

(event Input|ActionEvents|InputActionJump
  (params (Key :type Key%20Structure :default "None"))
  (bind _player (Variables|Default|GetPlayer))
  ;[1 1 1] Fall Through Floor
  (:Pressed
    (if (< (Input|AxisValues|GetMoveUp/Down) -0.5)
      (Character|StopJumping _player)
      (Default|FallThroughFloor _player "ECR_Ignore")
      (Pawn|Components|CharacterMovement|SetMovementMode (Variables|/Script/Engine.Character|GetCharacterMovement _player) "MOVE_Falling" 0))))

(fn ConstructionScript)