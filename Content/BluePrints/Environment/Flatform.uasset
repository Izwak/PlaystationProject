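; Moving platform actor that follows relative waypoints from LocationsVector through an InterpToMovement component.
; The construction script converts the waypoints into control points and sets the move duration from the distance between the first two points and a scaled Speed, printing it for debugging.
; BeginPlay appends the same points to the Locations array again without reassigning them to the component.
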(event EventBeginPlay
  (for _array_element (Variables|Default|GetLocationsVector)
    (Utilities|Array|Add (Variables|Default|GetLocations) (Utilities|Struct|MakeInterpControlPoint _array_element true))))

(fn ConstructionScript
  (bind _interptomovement (Variables|Default|GetInterpToMovement))
  (bind _locationsvector (Variables|Default|GetLocationsVector))
  (for _array_element (Variables|Default|GetLocationsVector)
    (Utilities|Array|Add (Variables|Default|GetLocations) (Utilities|Struct|MakeInterpControlPoint _array_element true))
    (Variables|/Script/Engine.InterpToMovementComponent|SetControlPoints _interptomovement (Variables|Default|GetLocations))
    (bind _output_get (Variables|/Script/Engine.InterpToMovementComponent|SetDuration _interptomovement (/ (Math|Vector|Distance(Vector) (Utilities|Array|Get(acopy) _locationsvector) (Utilities|Array|Get(acopy) _locationsvector 1)) (* (Variables|Default|GetSpeed) 2e+01))))
    (Development|PrintString (Utilities|String|ToString(Float) _output_get))))