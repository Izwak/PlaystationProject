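; Environment bush Blueprint that holds fruit the player can collect while standing next to it.
; On BeginPlay it gathers its Food child actors into an array and also records their transforms.
; The Box overlap toggles player input, so pressing Special destroys one fruit, increments the character's fruit and plays an eat sound.
; RemoveFruit and FruitCount provide bulk removal and the remaining count.
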(event OnComponentBeginOverlap(Box)
  (params (OverlappedComponent :type Primitive%20Component%20Object%20Reference) (OtherActor :type Actor%20Object%20Reference) (OtherComp :type Primitive%20Component%20Object%20Reference) (OtherBodyIndex :type Integer) (bFromSweep :type Boolean) (SweepResult :type Hit%20Result%20Structure%20%28by%20ref%29))
  ;[1 1 1] Enable Input
  (bind _asmy_character (Utilities|Casting|CastTomyCharacter OtherActor))
  (Input|EnableInput (Game|GetPlayerController 0))
  (Variables|Default|SetPlayerCharacter _asmy_character))

(event OnComponentEndOverlap(Box)
  (params (OverlappedComponent :type Primitive%20Component%20Object%20Reference) (OtherActor :type Actor%20Object%20Reference) (OtherComp :type Primitive%20Component%20Object%20Reference) (OtherBodyIndex :type Integer))
  ;[1 1 1] Enable Input
  (Utilities|Casting|CastTomyCharacter OtherActor)
  (Input|DisableInput (Game|GetPlayerController 0)))

(event Custom|RemoveFruit
  (params (RemoveNum :type Integer))
  (bind _fruits (Variables|Default|GetFruits))
  ;[1 1 1] Comment
  (for _index (range 0 RemoveNum)
    (Actor|DestroyActor (Utilities|Array|Get(acopy) _fruits))
    (Utilities|Array|RemoveIndex _fruits)))

(event EventBeginPlay
  ;[1 1 1] AddFruitToArray
  (for _array_element (Actor|GetAllChildActors true)
    (bind _asfood (Utilities|Casting|CastToFood _array_element))
    (Utilities|Array|Add (Variables|Default|GetFruits) _asfood)
    (Utilities|Array|Add (Variables|Default|GetFruitTransform) (Transformation|GetActorTransform _array_element))))

(event Input|ActionEvents|InputActionSpecial
  (params (Key :type Key%20Structure :default "None"))
  (bind _fruits (Variables|Default|GetFruits))
  (bind _playercharacter (Variables|Default|GetPlayerCharacter))
  (bind _returnvalue (Utilities|Array|Length _fruits))
  ;[1 1 1] Collect Fruit
  (:Pressed
    (if (> _returnvalue 0)
      (Actor|DestroyActor (Utilities|Array|Get(acopy) _fruits))
      (Utilities|Array|RemoveIndex _fruits)
      (Default|IncreaseFruit _playercharacter)
      (Audio|PlaySoundatLocation "/Game/Sounds/Eat.Eat" (Transformation|GetActorLocation _playercharacter) "0, 0, 0" 1.0 1.0 0.0 0 0 0 0)
      (Development|PrintString (Utilities|String|ToString(Integer) _returnvalue)))))

(fn ConstructionScript)

(fn FruitCount
  (return (Utilities|Array|Length (Variables|Default|GetFruits))))