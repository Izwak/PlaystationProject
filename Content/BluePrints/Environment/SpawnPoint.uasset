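; SpawnPoint is a lamp checkpoint that sets the player's respawn and last safe point to its location.
; Overlapping its collider enables input, so pressing Special activates it if unlit; a starting point activates itself shortly after BeginPlay.
; Activation darkens every SpawnPoint, lights this one through a dynamic material parameter, saves world state for the current level and fires a lightning effect.
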(event OnComponentBeginOverlap(Collider)
  (params (OverlappedComponent :type Primitive%20Component%20Object%20Reference) (OtherActor :type Actor%20Object%20Reference) (OtherComp :type Primitive%20Component%20Object%20Reference) (OtherBodyIndex :type Integer) (bFromSweep :type Boolean) (SweepResult :type Hit%20Result%20Structure%20%28by%20ref%29))
  ;[1 1 1] Can interact with
  (bind _asmy_character (Utilities|Casting|CastTomyCharacter OtherActor))
  (Input|EnableInput (Game|GetPlayerController 0))
  (Variables|Default|SetPlayer _asmy_character))

(event OnComponentEndOverlap(Collider)
  (params (OverlappedComponent :type Primitive%20Component%20Object%20Reference) (OtherActor :type Actor%20Object%20Reference) (OtherComp :type Primitive%20Component%20Object%20Reference) (OtherBodyIndex :type Integer))
  ;[1 1 1] Can interact with
  (Utilities|Casting|CastTomyCharacter OtherActor)
  (Input|DisableInput (Game|GetPlayerController 0)))

(event Custom|Un%20Lit
  ;[1 1 1] Lights Out
  (Variables|Default|SetisLit false)
  (Rendering|Material|SetScalarParameterValue (Variables|Default|GetLightMat) "Lighting" 0.0 :!class /Script/Engine.MaterialInstanceDynamic))

(event Custom|SetSafePoint
  ;[1 1 1] Check
  (Variables|/Game/Characters/Player/myCharacter.myCharacter_C|SetLastSafePoint (Variables|Default|GetPlayer) (Transformation|GetActorLocation)))

(event EventBeginPlay
  ;[1 1 1] Set Starting Spawn Point
  (Utilities|FlowControl|Delay 0.1)
  (bind _returnvalue (Rendering|Material|CreateDynamicMaterialInstance (Variables|Default|GetsavePoint) 0 "/Game/Objects/SavePoint/Material/LampOnMat.LampOnMat" "None" :!class /Script/Engine.PrimitiveComponent))
  (Variables|Default|SetLightMat _returnvalue)
  ;[1 1 1] Turn off all other lights and this light on
  (if (Variables|Default|GetisStartingPoint)
    (bind _asmy_character (Utilities|Casting|CastTomyCharacter (Game|GetPlayerCharacter 0)))
    (Variables|Default|SetPlayer _asmy_character)
    (Utilities|FlowControl|Delay 0.1)
    (Utilities|FlowControl|Sequence
      (:then_0
        ;;[1 1 1] Turn other Respawn Lights Off
        (bind _outactors (Actor|GetAllActorsOfClass "SpawnPoint_C"))
        (for _array_element _outactors
          (CallFunction|UnLit _array_element)))
      (:then_1
        ;;[1 1 1] Turn this light on
        (Development|PrintString "LightBoiBoi")
        (Variables|Default|SetisLit true)
        (Rendering|Material|SetScalarParameterValue (Variables|Default|GetLightMat) "Lighting" 15.0 :!class /Script/Engine.MaterialInstanceDynamic)
        (bind _returnvalue_2 (Game|GetCurrentLevelName true))
        (CallFunction|SaveWorldState _returnvalue_2))
      (:then_2
        ;;[1 1 1] Update Respawn Point
        (Default|SetRespawn (Variables|Default|GetPlayer) (Transformation|GetActorLocation))
        (Components|Activation|Activate (Variables|Default|GetP_ky_lightning1) false)
        (CallFunction|SetSafePoint)))))

(event Input|ActionEvents|InputActionSpecial
  (params (Key :type Key%20Structure :default "None"))
  ;[1 1 1] Turn off all other lights and this light on
  (:Pressed
    (if (not (Variables|Default|GetisLit))
      (Utilities|FlowControl|Sequence
        (:then_0
          ;;[1 1 1] Turn other Respawn Lights Off
          (bind _outactors (Actor|GetAllActorsOfClass "SpawnPoint_C"))
          (for _array_element _outactors
            (CallFunction|UnLit _array_element)))
        (:then_1
          ;;[1 1 1] Turn this light on
          (Development|PrintString "LightBoiBoi")
          (Variables|Default|SetisLit true)
          (Rendering|Material|SetScalarParameterValue (Variables|Default|GetLightMat) "Lighting" 15.0 :!class /Script/Engine.MaterialInstanceDynamic)
          (bind _returnvalue (Game|GetCurrentLevelName true))
          (CallFunction|SaveWorldState _returnvalue))
        (:then_2
          ;;[1 1 1] Update Respawn Point
          (Default|SetRespawn (Variables|Default|GetPlayer) (Transformation|GetActorLocation))
          (Components|Activation|Activate (Variables|Default|GetP_ky_lightning1) false)
          (CallFunction|SetSafePoint))))))

(fn ConstructionScript)