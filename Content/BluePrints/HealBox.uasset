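; HealBox is a trigger volume that gradually heals a myCharacter while it stands inside the Box.
; Begin overlap caches the character and starts a looping timer, using a negative start delay intended to make the first tick immediate.
; Each tick adds a fixed amount to Health, caps it at a hardcoded maximum and prints the result.
; End overlap by a myCharacter clears the timer.
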(event OnComponentBeginOverlap(Box)
  (params (OverlappedComponent :type Primitive%20Component%20Object%20Reference) (OtherActor :type Actor%20Object%20Reference) (OtherComp :type Primitive%20Component%20Object%20Reference) (OtherBodyIndex :type Integer) (bFromSweep :type Boolean) (SweepResult :type Hit%20Result%20Structure%20%28by%20ref%29))
  ;[1 1 1] Heal Player
  (bind _asmy_character (Utilities|Casting|CastTomyCharacter OtherActor))
  (Variables|Default|SetAs%20My%20Character _asmy_character)
  (bind _returnvalue (Utilities|Time|SetTimerbyEvent (delegate Custom|Heal) 0.2 true -0.2))
  (Variables|Default|SettimerRef _returnvalue))

(event OnComponentEndOverlap(Box)
  (params (OverlappedComponent :type Primitive%20Component%20Object%20Reference) (OtherActor :type Actor%20Object%20Reference) (OtherComp :type Primitive%20Component%20Object%20Reference) (OtherBodyIndex :type Integer))
  ;[1 1 1] Heal Player
  (Utilities|Casting|CastTomyCharacter OtherActor)
  (Utilities|Time|ClearandInvalidateTimerbyHandle (Variables|Default|GettimerRef)))

(event Custom|Heal
  (bind _as_my_character (Variables|Default|GetAs%20My%20Character))
  ;[1 1 1] Heal Player
  (if (< (+ (Variables|/Game/Characters/TestCharacter/myCharacter.myCharacter_C|GetHealth (stale OnComponentBeginOverlap(Box) _asmy_character)) 2.0) 1e+02)
    (bind _output_get (Variables|/Game/Characters/TestCharacter/myCharacter.myCharacter_C|SetHealth _as_my_character (+ (Variables|/Game/Characters/TestCharacter/myCharacter.myCharacter_C|GetHealth (stale OnComponentBeginOverlap(Box) _asmy_character)) 2.0)))
    (Development|PrintString (Utilities|String|ToString(Float) _output_get))
    (else
      (bind _output_get_2 (Variables|/Game/Characters/TestCharacter/myCharacter.myCharacter_C|SetHealth _as_my_character 1e+02))
      (Development|PrintString (Utilities|String|ToString(Float) _output_get_2)))))

(fn ConstructionScript)