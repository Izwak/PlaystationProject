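; Projectile actor that damages and knocks back the player character on hit, then destroys itself.
; Its sphere's hit event casts to myCharacter to apply damage and knockback from the hit location.
; A Tick-driven timer lets it ignore non-player hits in its first moments and destroys it after a short lifetime.
; Debug strings print on each destroy path.
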(event OnComponentHit(Sphere)
  (params (HitComponent :type Primitive%20Component%20Object%20Reference) (OtherActor :type Actor%20Object%20Reference) (OtherComp :type Primitive%20Component%20Object%20Reference) (NormalImpulse :type Vector :default "0, 0, 0") (Hit :type Hit%20Result%20Structure%20%28by%20ref%29))
  ;[1 1 1] Projectile
  (bind _asmy_character (Utilities|Casting|CastTomyCharacter OtherActor)
    (:then
      (Game|Damage|ApplyDamage _asmy_character 2e+01 0 0)
      (Default|Knockback _asmy_character (.Location (Collision|BreakHitResult Hit)))
      (Development|PrintString "player death")
      (Actor|DestroyActor :!label _label))
    (:CastFailed
      (if (> (stale EventTick _output_get) 0.05)
        (Development|PrintString "not player death")
        (goto _label)))))

(event EventTick
  (params (DeltaSeconds :type Float%20%28single-precision%29))
  ;[1 1 1] Projectile
  (bind _output_get (Variables|Default|Settimer (+ DeltaSeconds (Variables|Default|Gettimer))))
  (if (> _output_get 2.0)
    (Development|PrintString "Timeout")
    (Actor|DestroyActor)))

(fn ConstructionScript)