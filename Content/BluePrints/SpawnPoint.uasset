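; SpawnPoint is a checkpoint actor that sets the player's respawn location and shows whether it is the active one.
; Overlapping its collider enables input on the actor, so pressing Special at an unlit point activates it; leaving disables input.
; Activation, which also runs on BeginPlay for the starting point, unlights every SpawnPoint, lights this one, passes its location to myCharacter and triggers a lightning effect.
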(event OnComponentBeginOverlap(Collider)
  (params (OverlappedComponent :type Primitive%20Component%20Object%20Reference) (OtherActor :type Actor%20Object%20Reference) (OtherComp :type Primitive%20Component%20Object%20Reference) (OtherBodyIndex :type Integer) (bFromSweep :type Boolean) (SweepResult :type Hit%20Result%20Structure%20%28by%20ref%29))
  ;[1 1 1] Can interact with
  (bind _asmy_character (Utilities|Casting|CastTomyCharacter OtherActor))
  (Input|EnableInput (Game|GetPlayerController 0))
  (Variables|Default|SetMyCharacter _asmy_character)
  (Development|PrintString "Hello"))

(event OnComponentEndOverlap(Collider)
  (params (OverlappedComponent :type Primitive%20Component%20Object%20Reference) (OtherActor :type Actor%20Object%20Reference) (OtherComp :type Primitive%20Component%20Object%20Reference) (OtherBodyIndex :type Integer))
  ;[1 1 1] Can interact with
  (Utilities|Casting|CastTomyCharacter OtherActor)
  (Input|DisableInput (Game|GetPlayerController 0)))

(event Custom|Un%20Lit
  ;[1 1 1] Lights Out
  (Rendering|Material|SetMaterial (Variables|Default|GetLight) 0 (Variables|Default|GetMaterial%20Unlit))
  (Variables|Default|SetisLit false))

(event EventBeginPlay
  ;[1 1 1] Turn off all other lights and this light on
  ;;[1 1 1] Set Starting Spawn Point
  (if (Variables|Default|GetisStartingPoint)
    (bind _asmy_character (Utilities|Casting|CastTomyCharacter (Game|GetPlayerCharacter 0)))
    (Variables|Default|SetMyCharacter _asmy_character)
    (Utilities|FlowControl|Sequence
      (:then_0
        ;;[1 1 1] Turn other Respawn Lights Off
        (bind _outactors (Actor|GetAllActorsOfClass "SpawnPoint_C"))
        (for _array_element _outactors
          (CallFunction|UnLit _array_element)))
      (:then_1
        ;;[1 1 1] Turn this light on
        (Development|PrintString "Hello")
        (Variables|Default|SetisLit true)
        (Rendering|Material|SetMaterial (Variables|Default|GetLight) 0 (Variables|Default|GetMaterial%20Lit)))
      (:then_2
        ;;[1 1 1] Update Respawn Point
        (Default|SetRespawn (Variables|Default|GetMyCharacter) (Transformation|GetActorLocation))
        (Components|Activation|Activate (Variables|Default|GetP_ky_lightning1) false)))))

(event Input|ActionEvents|InputActionSpecial
  (params (Key :type Key%20Structure :default "None"))
  ;[1 1 1] Turn off all other lights and this light on
  (:Pressed
    (if (not (Variables|Default|GetisLit))
      (Utilities|FlowControl|Sequence
        (:then_0
          ;;[1 1 1] Turn other Respawn Lights Off
          (bind _outactors (Actor|GetAllActorsOfClass "SpawnPoint_C"))
          (for _array_element _outactors
            (CallFunction|UnLit _array_element)))
        (:then_1
          ;;[1 1 1] Turn this light on
          (Development|PrintString "Hello")
          (Variables|Default|SetisLit true)
          (Rendering|Material|SetMaterial (Variables|Default|GetLight) 0 (Variables|Default|GetMaterial%20Lit)))
        (:then_2
          ;;[1 1 1] Update Respawn Point
          (Default|SetRespawn (Variables|Default|GetMyCharacter) (Transformation|GetActorLocation))
          (Components|Activation|Activate (Variables|Default|GetP_ky_lightning1) false))))))

(fn ConstructionScript)