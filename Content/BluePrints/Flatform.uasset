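; Flatform is a moving platform Blueprint that travels between two configurable locations through an InterpToMovement component.
; Its construction script builds two relative control points from the location variables.
; It derives the movement duration from the distance between them divided by a scaled Speed, so travel rate stays consistent regardless of path length.
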(fn ConstructionScript
  (bind _interptomovement (Variables|Default|GetInterpToMovement))
  (Variables|/Script/Engine.InterpToMovementComponent|SetControlPoints _interptomovement (Utilities|Array|MakeArray (Utilities|Struct|MakeInterpControlPoint (Variables|Default|GetLocation%201) true) (Utilities|Struct|MakeInterpControlPoint (Variables|Default|GetLocaition%202) true)))
  (Variables|/Script/Engine.InterpToMovementComponent|SetDuration _interptomovement (/ (Math|Vector|Distance(Vector) (Variables|Default|GetLocation%201) (Variables|Default|GetLocaition%202)) (* (Variables|Default|GetSpeed) 2e+01))))